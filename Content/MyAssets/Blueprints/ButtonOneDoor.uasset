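; ButtonOneDoor is a one-shot floor button that moves a linked door actor when something overlaps its trigger box.
; The first overlap lowers the button, swaps it to an activated material, plays a sound and activates a particle system.
; A timeline lerps the door from its start location, cached in the construction script, to that location plus PositionMove.
; When the timeline finishes, the button's particles and the Door's particle system are deactivated.
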(event OnComponentBeginOverlap(Box)
  (params (OverlappedComponent :type Primitive%20Component%20Object%20Reference) (OtherActor :type Actor%20Object%20Reference) (OtherComp :type Primitive%20Component%20Object%20Reference) (OtherBodyIndex :type Integer) (bFromSweep :type Boolean) (SweepResult :type Hit%20Result%20Structure%20%28by%20ref%29))
  (bind _button (Variables|Default|GetButton))
  (Utilities|FlowControl|DoOnce false
    (:Completed
      (Components|Activation|Activate (Variables|Default|GetParticleSystem1) false)
      (Transformation|AddLocalOffset _button "0, 0,-17.000000" false false)
      (Rendering|Material|SetMaterial _button 0 "/Game/MyAssets/Materials/Button_Activated.Button_Activated")
      (Audio|PlaySoundatLocation "/Game/FirstPerson/Audio/FirstPersonTemplateWeaponFire02.FirstPersonTemplateWeaponFire02" (Variables|Default|GetElementStart) "0, 0, 0" 1.0 1.0 0.0 0 0 0)
      (bind _track (Timeline|Timeline_0 PlayFromStart)
        (:Update
          (Transformation|SetActorLocation (Variables|Default|GetElementDoor) (Math|Vector|Lerp(Vector) (Variables|Default|GetElementStart) (Variables|Default|GetElementEnd) _track) false false))
        (:Finished
          (Components|Activation|Deactivate (Variables|Default|GetParticleSystem1))
          (Components|Activation|Deactivate (Variables|/Game/MyAssets/Blueprints/Door.Door_C|GetParticleSystem (.AsDoor (Utilities|Casting|CastToDoor (Variables|Default|GetElementDoor))))))))))

(fn ConstructionScript
  (bind _output_get (Variables|Default|SetElementStart (Transformation|GetActorLocation (Variables|Default|GetElementDoor))))
  (Variables|Default|SetElementEnd (+ _output_get (Variables|Default|GetPositionMove))))