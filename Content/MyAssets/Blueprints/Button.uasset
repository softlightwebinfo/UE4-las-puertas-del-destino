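; A pressure button that opens a linked door when something overlaps its trigger box.
; The IsDispatcher flag selects whether the overlap broadcasts the ClickButtonOpenDoor dispatcher or runs the OpenDoor event directly.
; OpenDoor fires once, activating particles, sinking the button mesh, swapping to the activated material and calling OpenDoor on ElementDoor through the IDoor interface.
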(event OnComponentBeginOverlap(Box)
  (params (OverlappedComponent :type Primitive%20Component%20Object%20Reference) (OtherActor :type Actor%20Object%20Reference) (OtherComp :type Primitive%20Component%20Object%20Reference) (OtherBodyIndex :type Integer) (bFromSweep :type Boolean) (SweepResult :type Hit%20Result%20Structure%20%28by%20ref%29))
  (if (Variables|Default|GetisDispatcher)
    (Default|CallClickButtonOpenDoor)
    (else
      (CallFunction|OpenDoor))))

(event Custom|OpenDoor
  (bind _button (Variables|Default|GetButton))
  (Utilities|FlowControl|DoOnce false
    (:Completed
      (Components|Activation|Activate (Variables|Default|GetParticleSystem1) false)
      (Transformation|AddLocalOffset _button "0, 0,-17.000000" false false)
      (Rendering|Material|SetMaterial _button 0 "/Game/MyAssets/Materials/Button_Activated.Button_Activated")
      (bind _asidoor (Utilities|Casting|CastToIDoor (Variables|Default|GetElementDoor)))
      (Default|OpenDoor _asidoor))))

(fn ConstructionScript)