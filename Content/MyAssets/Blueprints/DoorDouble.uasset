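; DoorDouble is a two-leaf door Blueprint that swings open when its OpenDoor event is called.
; The construction script stores each leaf's world rotation as the start and derives an end rotation with yaw set to absolute zero.
; OpenDoor plays a weapon-fire sound, drives a timeline that lerps both leaves along the shortest path, then deactivates a particle system when finished.
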(event EventOpenDoor
  (Audio|PlaySoundatLocation "/Game/FirstPerson/Audio/FirstPersonTemplateWeaponFire02.FirstPersonTemplateWeaponFire02" (Transformation|GetActorLocation) "0, 0, 0" 1.0 1.0 0.0 0 0 0)
  (bind _track (Timeline|Timeline_0 PlayFromStart)
    (:Update
      (Transformation|SetWorldRotation (Variables|Default|GetDoorLeft) (Math|Rotator|Lerp(Rotator) (Variables|Default|GetDoorLeftStart) (Variables|Default|GetDoorLeftEnd) _track true) false false)
      (Transformation|SetWorldRotation (Variables|Default|GetDoorRight) (Math|Rotator|Lerp(Rotator) (Variables|Default|GetDoorRightStart) (Variables|Default|GetDoorRightEnd) _track true) false false))
    (:Finished
      (Components|Activation|Deactivate (Variables|Default|GetParticleSystem)))))

(fn ConstructionScript
  (Variables|Default|SetDoorRightStart (Transformation|GetWorldRotation (Variables|Default|GetDoorRight)))
  (Variables|Default|SetDoorLeftStart (Transformation|GetWorldRotation (Variables|Default|GetDoorLeft)))
  (Variables|Default|SetDoorRightEnd (Math|Rotator|MakeRotator (.Roll (Math|Rotator|BreakRotator (Variables|Default|GetDoorRightStart))) (.Pitch (Math|Rotator|BreakRotator (Variables|Default|GetDoorRightStart))) 0.0))
  (Variables|Default|SetDoorLeftEnd (Math|Rotator|MakeRotator (.Roll (Math|Rotator|BreakRotator (Variables|Default|GetDoorLeftStart))) (.Pitch (Math|Rotator|BreakRotator (Variables|Default|GetDoorLeftStart))) 0.0)))